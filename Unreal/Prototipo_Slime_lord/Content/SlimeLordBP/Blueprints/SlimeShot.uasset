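; SlimeShot is a cone pickup that grants the third-person character one ShotSlimes charge on overlap, only when its count is zero.
; The overlap stores the character reference and prints the new count in green.
; Tick polls that count through the stored reference, hiding the cone and disabling collision while it is above zero, and restoring both otherwise.
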(event `self.ReceiveTick`
  (params (DeltaSeconds :type "Float (single-precision)"))
  (bind _cone (`self.Cone`))
  (if (> (`/Game/SlimeLordBP/Blueprints/ThirdPersonCharacter.ShotSlimes` (stale `self.ReceiveActorBeginOverlap` _asthird_person_character)) 0)
    (`self.SetActorEnableCollision` false)
    (`SceneComponent.SetHiddenInGame` _cone true false)
    (else
      (`self.SetActorEnableCollision` true)
      (`SceneComponent.SetHiddenInGame` _cone false false))))

(event `self.ReceiveActorBeginOverlap`
  (params (OtherActor :type "Actor Object Reference"))
  (bind _asthird_person_character (cast `/Game/SlimeLordBP/Blueprints/ThirdPersonCharacter` OtherActor))
  (bind _shotslimes (`/Game/SlimeLordBP/Blueprints/ThirdPersonCharacter.ShotSlimes` _asthird_person_character))
  (if (== _shotslimes 0)
    (bind _output_get (set `/Game/SlimeLordBP/Blueprints/ThirdPersonCharacter.ShotSlimes` (+ _shotslimes 1) _asthird_person_character))
    (`KismetSystemLibrary.PrintString` (`KismetStringLibrary.Conv_IntToString` _output_get) true true (struct :`R` 0.10871 :`G` 1.0 :`A` 1.0))))

(fn `UserConstructionScript`)