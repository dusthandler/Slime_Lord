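; SlimeShot is a pickup that adds one to the ThirdPersonCharacter's ShotSlimes count when that character overlaps it.
; On pickup it stores the new count in MaxSlimes, prints it, then disables collision and hides its Cone.
; A five-second Delay loop re-checks the count and restores the pickup only once ShotSlimes has dropped below the stored value.
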(event `self.ReceiveActorBeginOverlap`
  (params (OtherActor :type "Actor Object Reference"))
  ;[1 1 1] Incrementa cantidad de Slimes
  (bind _asthird_person_character (cast `/Game/SlimeLordBP/Blueprints/ThirdPersonCharacter` OtherActor))
  (bind _shotslimes (`/Game/SlimeLordBP/Blueprints/ThirdPersonCharacter.ShotSlimes` _asthird_person_character))
  (bind _output_get (set `/Game/SlimeLordBP/Blueprints/ThirdPersonCharacter.ShotSlimes` (+ _shotslimes 1) _asthird_person_character))
  (set `self.MaxSlimes` _output_get)
  (`KismetSystemLibrary.PrintString` (`KismetStringLibrary.Conv_IntToString` _output_get) true true (struct :`G` 1.0 :`B` 0.106406 :`A` 1.0))
  ;[1 1 1] Desactiva colisionador y visivilidad de slimes y los reactiva pasado un tiempo (falta condicion de que no reaparezca si aun no has gastado ese slime)
  (`self.SetActorEnableCollision` false)
  (`SceneComponent.SetHiddenInGame` (`self.Cone`) true false)
  (`KismetSystemLibrary.Delay` 5.0 :!label _label)
  (if (< _shotslimes (`self.MaxSlimes`))
    (`self.SetActorEnableCollision` true)
    (`SceneComponent.SetHiddenInGame` (`self.Cone`) false false)
    (else
      (goto _label))))

(fn `UserConstructionScript`)