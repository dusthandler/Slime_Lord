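; Axe trap actor that swings two axes and damages the player when it registers a hit.
; On BeginPlay, two timelines each drive the world pitch of a scene component, keeping the actor's roll and yaw.
; Any Hit event subtracts one Health from player 0's ThirdPersonCharacter, without checking which actor was hit.
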(event `self.ReceiveHit`
  (params (MyComp :type "PrimitiveComponent Object Reference") (Other :type "Actor Object Reference") (OtherComp :type "PrimitiveComponent Object Reference") (bSelfMoved :type Boolean) (HitLocation :type "Vector Structure") (HitNormal :type "Vector Structure") (NormalImpulse :type "Vector Structure") (Hit :type "HitResult Structure (by ref)"))
  (bind _asthird_person_character (cast `/Game/SlimeLordBP/Blueprints/ThirdPersonCharacter` (`GameplayStatics.GetPlayerCharacter` 0)))
  (set `/Game/SlimeLordBP/Blueprints/ThirdPersonCharacter.Health` (- (`/Game/SlimeLordBP/Blueprints/ThirdPersonCharacter.Health` _asthird_person_character) 1.0) _asthird_person_character))

(event `self.ReceiveBeginPlay`
  (bind (_returnvalue_roll _returnvalue_pitch _returnvalue_yaw) (`KismetMathLibrary.BreakRotator` (`self.K2_GetActorRotation`)))
  (bind (_returnvalue_roll_2 _returnvalue_pitch_2 _returnvalue_yaw_2) (`KismetMathLibrary.BreakRotator` (`self.K2_GetActorRotation`)))
  (`|ExecutionSequence`
    (:`then_0`
      (bind (_direction _rotation) (`Timeline|Hacha1Movement`)
        (:`Update`
          (`SceneComponent.K2_SetWorldRotation` (`self.Scene1`) (`KismetMathLibrary.MakeRotator` _returnvalue_roll _rotation _returnvalue_yaw) false false))))
    (:`then_1`
      (bind (_direction_2 _rotation_2) (`Timeline|Hacha2Movement`)
        (:`Update`
          (`SceneComponent.K2_SetWorldRotation` (`self.Scene2`) (`KismetMathLibrary.MakeRotator` _returnvalue_roll_2 _rotation_2 _returnvalue_yaw_2) false false))))))

(fn `UserConstructionScript`)