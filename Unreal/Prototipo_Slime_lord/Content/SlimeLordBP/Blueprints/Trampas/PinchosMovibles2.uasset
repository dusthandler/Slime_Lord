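; Moving spike trap actor that damages the player and travels along the vertical axis.
; On BeginPlay, the PinchosArriba timeline sets the Platform component's world position to the actor's location plus an animated Z offset.
; Any Hit event subtracts one Health from player 0's ThirdPersonCharacter, without checking which actor made contact.
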(event `self.ReceiveHit`
  (params (MyComp :type "PrimitiveComponent Object Reference") (Other :type "Actor Object Reference") (OtherComp :type "PrimitiveComponent Object Reference") (bSelfMoved :type Boolean) (HitLocation :type "Vector Structure") (HitNormal :type "Vector Structure") (NormalImpulse :type "Vector Structure") (Hit :type "HitResult Structure (by ref)"))
  ;[1 1 1] Daño
  (bind _asthird_person_character (cast `/Game/SlimeLordBP/Blueprints/ThirdPersonCharacter` (`GameplayStatics.GetPlayerCharacter` 0)))
  (set `/Game/SlimeLordBP/Blueprints/ThirdPersonCharacter.Health` (- (`/Game/SlimeLordBP/Blueprints/ThirdPersonCharacter.Health` _asthird_person_character) 1.0) _asthird_person_character))

(event `self.ReceiveBeginPlay`
  (bind (_returnvalue_x _returnvalue_y _returnvalue_z) (`KismetMathLibrary.BreakVector` (`self.K2_GetActorLocation`)))
  ;[1 1 1] Movimiento
  (bind (_direction _pinchosup) (`Timeline|PinchosArriba`)
    (:`Update`
      (`SceneComponent.K2_SetWorldLocation` (`self.Platform`) (`KismetMathLibrary.MakeVector` _returnvalue_x _returnvalue_y (+ _returnvalue_z _pinchosup)) false false))))

(fn `UserConstructionScript`)