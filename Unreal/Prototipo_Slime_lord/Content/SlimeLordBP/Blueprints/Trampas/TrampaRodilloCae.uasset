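; Falling roller trap that takes one Health from player 0's ThirdPersonCharacter whenever anything begins overlapping its Collision component.
; A separate Box overlap only sets OnOverlap.
; The Construction Script loads three relative locations and a Duration into InterpToMovement inside a while loop on that flag, so the runtime overlap does not itself trigger movement.
; A delayed copy of that movement setup sits unconnected in the EventGraph.
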(event `self.Collision.OnComponentBeginOverlap`
  (params (OverlappedComponent :type "PrimitiveComponent Object Reference") (OtherActor :type "Actor Object Reference") (OtherComp :type "PrimitiveComponent Object Reference") (OtherBodyIndex :type Integer) (bFromSweep :type Boolean) (SweepResult :type "HitResult Structure (by ref)"))
  ;[1 1 1] Daño
  (bind _asthird_person_character (cast `/Game/SlimeLordBP/Blueprints/ThirdPersonCharacter` (`GameplayStatics.GetPlayerCharacter` 0)))
  (set `/Game/SlimeLordBP/Blueprints/ThirdPersonCharacter.Health` (- (`/Game/SlimeLordBP/Blueprints/ThirdPersonCharacter.Health` _asthird_person_character) 1.0) _asthird_person_character))

(event `self.Box.OnComponentBeginOverlap`
  (params (OverlappedComponent :type "PrimitiveComponent Object Reference") (OtherActor :type "Actor Object Reference") (OtherComp :type "PrimitiveComponent Object Reference") (OtherBodyIndex :type Integer) (bFromSweep :type Boolean) (SweepResult :type "HitResult Structure (by ref)"))
  (set `self.OnOverlap` true))

(fn `UserConstructionScript`
  (bind _interptomovement (`self.InterpToMovement`))
  ;[1 1 1] Movimiento
  (while (`self.OnOverlap`)
    (set `InterpToMovementComponent.ControlPoints` (`|MakeArray` (make `InterpControlPoint` (`self.Location1`)) (make `InterpControlPoint` (`self.location2`)) (make `InterpControlPoint` (`self.Location3`))) _interptomovement)
    (set `InterpToMovementComponent.Duration` (`self.duration`) _interptomovement)))