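; AguaTrampa is a water trap that rises once the player has stepped on two pistons and damages the player on overlap.
; BeginPlay polls the player character's PistonsStepped every 0.1 seconds, then plays the AguaSubida timeline to lift the Cube from the actor's location.
; A long delay off the timeline update later stops it.
; Any overlap with Collision subtracts Health from the player character, whichever actor triggered it.
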(event `self.Collision.OnComponentBeginOverlap`
  (params (OverlappedComponent :type "PrimitiveComponent Object Reference") (OtherActor :type "Actor Object Reference") (OtherComp :type "PrimitiveComponent Object Reference") (OtherBodyIndex :type Integer) (bFromSweep :type Boolean) (SweepResult :type "HitResult Structure (by ref)"))
  ;[1 1 1] Daño
  (bind _asthird_person_character (cast `/Game/SlimeLordBP/Blueprints/ThirdPersonCharacter` (`GameplayStatics.GetPlayerCharacter` 0)))
  (set `/Game/SlimeLordBP/Blueprints/ThirdPersonCharacter.Health` (- (`/Game/SlimeLordBP/Blueprints/ThirdPersonCharacter.Health` _asthird_person_character) 1.0) _asthird_person_character))

(event `self.ReceiveBeginPlay`
  (bind (_returnvalue_x _returnvalue_y _returnvalue_z) (`KismetMathLibrary.BreakVector` (`self.K2_GetActorLocation`)))
  ;[1 1 1] Movimiento
  (bind _asthird_person_character (cast `/Game/SlimeLordBP/Blueprints/ThirdPersonCharacter` (`GameplayStatics.GetPlayerCharacter` 0) :!label _label))
  (if (== (`/Game/SlimeLordBP/Blueprints/ThirdPersonCharacter.PistonsStepped` _asthird_person_character) 2)
    (`KismetSystemLibrary.PrintString` "agua sube")
    (bind (_direction _aguaup) (`Timeline|AguaSubida` :!label _label_2)
      (:`Update`
        (`SceneComponent.K2_SetWorldLocation` (`self.Cube`) (`KismetMathLibrary.MakeVector` _returnvalue_x _returnvalue_y (+ _returnvalue_z _aguaup)) false false)
        (`KismetSystemLibrary.Delay` 240.0)
        (goto _label_2 :!via `Stop`)))
    (else
      (`KismetSystemLibrary.Delay` 0.1)
      (goto _label))))

(fn `UserConstructionScript`)