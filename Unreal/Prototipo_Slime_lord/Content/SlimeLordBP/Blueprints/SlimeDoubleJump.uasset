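; SlimeDoubleJump is a slime pickup that grants jump charges to the ThirdPersonCharacter.
; On overlap it stores the character, increments JumpSlimes, copies that count to JumpCont and prints it.
; Tick polls the stored character's JumpSlimes, hiding the Cone and disabling collision while it is above zero and restoring both otherwise, so the pickup reappears rather than being destroyed.
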(event `self.ReceiveTick`
  (params (DeltaSeconds :type "Float (single-precision)"))
  (bind _cone (`self.Cone`))
  (if (> (`/Game/SlimeLordBP/Blueprints/ThirdPersonCharacter.JumpSlimes` (stale `self.ReceiveActorBeginOverlap` _asthird_person_character)) 0)
    (`self.SetActorEnableCollision` false)
    (`SceneComponent.SetHiddenInGame` _cone true false)
    (else
      (`self.SetActorEnableCollision` true)
      (`SceneComponent.SetHiddenInGame` _cone false false))))

(event `self.ReceiveActorBeginOverlap`
  (params (OtherActor :type "Actor Object Reference"))
  (bind _asthird_person_character (cast `/Game/SlimeLordBP/Blueprints/ThirdPersonCharacter` OtherActor))
  (bind _jumpslimes (`/Game/SlimeLordBP/Blueprints/ThirdPersonCharacter.JumpSlimes` _asthird_person_character))
  (bind _output_get (set `/Game/SlimeLordBP/Blueprints/ThirdPersonCharacter.JumpSlimes` (+ _jumpslimes 1) _asthird_person_character))
  (`KismetSystemLibrary.PrintString` (`KismetStringLibrary.Conv_IntToString` _output_get))
  (set `/Game/SlimeLordBP/Blueprints/ThirdPersonCharacter.JumpCont` _jumpslimes _asthird_person_character))

(fn `UserConstructionScript`)