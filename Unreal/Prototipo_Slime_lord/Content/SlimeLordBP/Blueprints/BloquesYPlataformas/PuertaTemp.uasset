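; PuertaTemp is a timed door that moves vertically when the level's DianaTemp (target) actor sets OpenDoor.
; From BeginPlay it polls the first DianaTemp found every 0.2 seconds, then plays the PuertaFall timeline to drive the door's world Z.
; A TempDoor state counter, advanced inside the timeline's Update, uses delays to stop the movement, hold, reverse and return to polling.
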(event `self.ReceiveBeginPlay`
  (bind (_returnvalue_x _returnvalue_y) (`KismetMathLibrary.BreakVector` (`self.K2_GetActorLocation`)))
  (bind _outactors (`GameplayStatics.GetAllActorsOfClass` "/Game/SlimeLordBP/Blueprints/BloquesYPlataformas/DianaTemp.DianaTemp_C" :!label _label))
  (bind _asdiana_temp (cast `/Game/SlimeLordBP/Blueprints/BloquesYPlataformas/DianaTemp` (`|GetArrayItem` _outactors)))
  (if (`/Game/SlimeLordBP/Blueprints/BloquesYPlataformas/DianaTemp.OpenDoor` _asdiana_temp)
    (bind (_direction _doorfall) (`Timeline|PuertaFall` :!label _label_2)
      (:`Update`
        (`self.K2_SetActorLocation` (`KismetMathLibrary.MakeVector` _returnvalue_x _returnvalue_y _doorfall))
        (if (== (`self.TempDoor`) 0)
          (set `self.TempDoor` 1)
          ;[1 1 1] Tiempo movimiento puerta
          (`KismetSystemLibrary.Delay` 6.0)
          (goto _label_2 :!via `Stop`)
          (elif (== (`self.TempDoor`) 1)
            ;[1 1 1] tiempo puerta quieta
            (`KismetSystemLibrary.Delay` 6.0)
            (set `self.TempDoor` 2)
            (goto _label_2 :!via `Reverse`)
            (else
              (set `self.TempDoor` 0)
              (`KismetSystemLibrary.Delay` 0.2 :!label _label_3)
              (goto _label))))))
    (else
      (goto _label_3))))

(fn `UserConstructionScript`)